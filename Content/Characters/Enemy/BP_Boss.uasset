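; BP_Boss is a boss enemy character that runs the BT_Boss behavior tree on its AI controller from BeginPlay.
; Pawn sensing passes seen pawns and the player pawn to DetectPawn, then creates a new WBP_Boss health widget on every sighting.
; Damage reduces health through StatsComp, whose percentage delegate updates that widget.
; Select and deselect events toggle the lock-on marker.
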(event `self.ReceiveBeginPlay`
  (`AIController.RunBehaviorTree` (`AIBlueprintHelperLibrary.GetAIController` self) "/Game/Characters/AI/BT_Boss.BT_Boss"))

(event `self.OnSelect`
  (`SceneComponent.SetVisibility` (`self.Lockon Widget`) true false))

(event `self.OnDeselect`
  (`SceneComponent.SetVisibility` (`self.Lockon Widget`) false false))

(event `self.ReceiveAnyDamage`
  (params (Damage :type "Float (single-precision)") (DamageType :type "DamageType Object Reference") (InstigatedBy :type "Controller Object Reference") (DamageCauser :type "Actor Object Reference"))
  (`StatsComponent.ReduceHealth` (`self.StatsComp`) Damage))

(event `self.PawnSensing.OnSeePawn`
  (params (Pawn :type "Pawn Object Reference"))
  (`self.DetectPawn` Pawn (`GameplayStatics.GetPlayerPawn` 0))
  (bind _returnvalue (`|CreateWidget` "/Game/UI/WBP_Boss.WBP_Boss_C"))
  (bind _output_get (set `self.Boss Widget` _returnvalue))
  (`UserWidget.AddToViewport` _output_get 0)
  (`/Game/UI/WBP_Boss.SetHealthPercentage` (`self.Boss Widget`) (`StatsComponent.GetStatPercentage` (`self.StatsComp`) "Health" "MaxHealth")))

(event `self.StatsComp.OnHealthPercentUpdateDelegate`
  (params (Percentage :type "Float (single-precision)"))
  (`/Game/UI/WBP_Boss.SetHealthPercentage` (`self.Boss Widget`) Percentage))

(fn `UserConstructionScript`)